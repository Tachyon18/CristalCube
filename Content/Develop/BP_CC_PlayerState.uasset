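; Player state Blueprint that provides a function to open the skill inventory UI.
; CreateInventoryWidget returns true if the widget already exists; otherwise it creates WBP_SkillInventory for player controller 0, adds it to the viewport and returns false.
; BeginPlay and Tick are empty.
; Disconnected leftover nodes would grant spell skills such as BP_FireBall and BP_MeteorShower, or remove the inventory from its parent, but never run.
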(event EventBeginPlay)

(event EventTick
  (params (DeltaSeconds :type Float%20%28single-precision%29)))

(fn ConstructionScript)

(fn CreateInventoryWidget
  (if (Utilities|IsValid (Variables|Default|GetSkillInventory))
    (return true)
    (else
      (bind _returnvalue (UserInterface|CreateWidget "/Game/Develop/Widget/WBP_SkillInventory.WBP_SkillInventory_C" (Game|GetPlayerController 0)))
      (bind _output_get (Variables|Default|SetSkillInventory _returnvalue))
      (UserInterface|Viewport|AddtoViewport _output_get 0)
      (return false))))